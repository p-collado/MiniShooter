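; AI controller for shooter enemies that chases the player and jumps upon getting close.
; On BeginPlay it grants the GA_Jump ability to the possessed BP_Enemy through its Ability System Component and keeps the handle.
; Tick re-issues a MoveToLocation toward player 0 with an acceptance radius.
; A DoOnce activates the jump when already at goal and re-arms when a new move request succeeds.
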(event `self.ReceiveBeginPlay`
  (bind _asbp_enemy (cast `/Game/Blueprint/IA/BP_Enemy` (`self.K2_GetPawn`)))
  (bind _returnvalue (`AbilitySystemComponent.K2_GiveAbility` (`ShooterEnemy.AbilitySystemComponent` _asbp_enemy) "/Game/GAS/CharacterAbilities/GA_Jump.GA_Jump_C" 0 -1)))

(event `self.ReceiveTick`
  (params (DeltaSeconds :type "Float (single-precision)"))
  (bind _returnvalue (`self.MoveToLocation` (`self.K2_GetActorLocation` (`GameplayStatics.GetPlayerCharacter` 0)) 300.0 true true false true null))
  (switch `EPathFollowingRequestResult` _returnvalue
    (:`AlreadyAtGoal`
      (`/Engine/EditorBlueprintResources/StandardMacros.DoOnce` false :!label _label
        (:`Completed`
          (bind _asbp_enemy (cast `/Game/Blueprint/IA/BP_Enemy` (`self.K2_GetPawn`)))
          (`AbilitySystemComponent.TryActivateAbility` (`ShooterEnemy.AbilitySystemComponent` _asbp_enemy) (stale `self.ReceiveBeginPlay` _returnvalue) true))))
    (:`RequestSuccessful`
      (goto _label :!via `Reset`))))

(fn `UserConstructionScript`)