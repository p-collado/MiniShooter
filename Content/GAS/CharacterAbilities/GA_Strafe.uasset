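; GA_Strafe is a hold-to-strafe Gameplay Ability that switches the player to controller-facing movement until input is released.
; On activation it raises the player AnimBP's strafe alpha, pulls in and shifts the camera, and applies GE_SlowDown via SetByCaller magnitude.
; OnEndAbility reverses these, reapplying GE_SlowDown with a higher magnitude instead of removing it.
; The enemy AnimBP activation branch is an empty stub.
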(event `self.K2_ActivateAbility`
  (bind (_returnvalue_owneractor _returnvalue_avataractor) (break `GameplayAbilityActorInfo` (`self.GetActorInfo`)))
  (bind (_returnvalue_owneractor_2 _returnvalue_avataractor_2) (break `GameplayAbilityActorInfo` (`self.GetActorInfo`)))
  (`self.K2_CommitAbility`)
  (bind _ascharacter_base (cast `CharacterBase` _returnvalue_avataractor)
    (:`then`
      (if (`KismetSystemLibrary.IsValid` _ascharacter_base)
        (bind _returnvalue (`SkeletalMeshComponent.GetAnimInstance` (`Character.Mesh` _ascharacter_base)))
        ;[1 1 1] TODO: Cambiar strafe a template
        (bind _asabp_player (cast `/Game/Animations/Character/ABP_Player` _returnvalue)
          (:`then`
            (if (`KismetSystemLibrary.IsValid` _asabp_player)
              (set `/Game/Animations/Character/ABP_Player.AlphaStrafe` 1.0 _asabp_player)
              (bind _ascharacter_base_2 (cast `CharacterBase` _returnvalue_avataractor_2)
                (:`then`
                  (if (`KismetSystemLibrary.IsValid` _ascharacter_base_2)
                    (bind _charactermovement (`Character.CharacterMovement` _ascharacter_base_2))
                    (set `CharacterMovementComponent.bOrientRotationToMovement` false _charactermovement)
                    (set `CharacterMovementComponent.bUseControllerDesiredRotation` true _charactermovement)
                    (bind _asbp_player_character (cast `/Game/Blueprint/Character/BP_PlayerCharacter` _ascharacter_base_2)
                      (:`then`
                        (set `SpringArmComponent.TargetArmLength` 200.0 (`PlayerCharacter.CameraBoom` _asbp_player_character))
                        (`SceneComponent.K2_SetRelativeLocation` (`PlayerCharacter.FollowCamera` _asbp_player_character) (100.0 50.0 100.0) false false))
                      (:`CastFailed`
                        _))
                    (bind _returnvalue_2 (`AbilitySystemBlueprintLibrary.AssignTagSetByCallerMagnitude` (`self.MakeOutgoingGameplayEffectSpec` "/Game/GAS/GameplayEffects/GE_SlowDown.GE_SlowDown_C") (struct :`TagName` "Effect.Slow.Strafe") 400.0))
                    (`self.K2_ApplyGameplayEffectSpecToOwner` _returnvalue_2)
                    (`AbilityTask_WaitInputRelease.WaitInputRelease` false
                      (:`OnRelease`
                        (`self.K2_EndAbility`)))
                    (else
                      (`KismetSystemLibrary.PrintString` "invalid character")
                      (`self.K2_EndAbility` :!label _label))))
                (:`CastFailed`
                  (`KismetSystemLibrary.PrintString` "Error Casteo personaje")
                  (goto _label)))
              (else
                (`KismetSystemLibrary.PrintString` "No valido" :!label _label_2)
                (goto _label))))
          (:`CastFailed`
            (bind _asabp_enemy (cast `/Game/Animations/Crypto/ABP_Enemy` _returnvalue)
              (:`then`
                (if (`KismetSystemLibrary.IsValid` _asabp_enemy)
                  _))
              (:`CastFailed`
                (`KismetSystemLibrary.PrintString` "anim instance fail")
                (goto _label)))))
        (else
          (goto _label_2))))
    (:`CastFailed`
      (`KismetSystemLibrary.PrintString` "Error castep")
      (goto _label))))

(event `self.K2_OnEndAbility`
  (params (bWasCancelled :type Boolean))
  (bind (_returnvalue_owneractor _returnvalue_avataractor) (break `GameplayAbilityActorInfo` (`self.GetActorInfo`)))
  (bind (_returnvalue_owneractor_2 _returnvalue_avataractor_2) (break `GameplayAbilityActorInfo` (`self.GetActorInfo`)))
  (bind _ascharacter_base (cast `CharacterBase` _returnvalue_avataractor)
    (:`then`
      (if (`KismetSystemLibrary.IsValid` _ascharacter_base)
        (bind _returnvalue (`SkeletalMeshComponent.GetAnimInstance` (`Character.Mesh` _ascharacter_base)))
        ;[1 1 1] TODO: CAMBIAR A INTERFACE
        (bind _asabp_player (cast `/Game/Animations/Character/ABP_Player` _returnvalue)
          (:`then`
            (if (or (`KismetSystemLibrary.IsValid` (stale _asabp_enemy)) (`KismetSystemLibrary.IsValid` _asabp_player)) :!label _label_3
              (set `/Game/Animations/Character/ABP_Player.AlphaStrafe` 0.0 _asabp_player)
              (bind _ascharacter_base_2 (cast `CharacterBase` _returnvalue_avataractor_2)
                (:`then`
                  (if (`KismetSystemLibrary.IsValid` _ascharacter_base_2)
                    (bind _charactermovement (`Character.CharacterMovement` _ascharacter_base_2))
                    (set `CharacterMovementComponent.bOrientRotationToMovement` true _charactermovement)
                    (set `CharacterMovementComponent.bUseControllerDesiredRotation` false _charactermovement)
                    (bind _asbp_player_character (cast `/Game/Blueprint/Character/BP_PlayerCharacter` _ascharacter_base_2)
                      (:`then`
                        (set `SpringArmComponent.TargetArmLength` 400.0 (`PlayerCharacter.CameraBoom` _asbp_player_character))
                        (`SceneComponent.K2_SetRelativeLocation` (`PlayerCharacter.FollowCamera` _asbp_player_character) (100.0 -3.0 96.0) false false)
                        (bind _returnvalue_2 (`AbilitySystemBlueprintLibrary.AssignTagSetByCallerMagnitude` (`self.MakeOutgoingGameplayEffectSpec` "/Game/GAS/GameplayEffects/GE_SlowDown.GE_SlowDown_C") (struct :`TagName` "Effect.Slow.Strafe") 600.0))
                        (`self.K2_ApplyGameplayEffectSpecToOwner` _returnvalue_2))
                      (:`CastFailed`
                        (`KismetSystemLibrary.PrintString` "invalid character" :!label _label_4)))
                    (else
                      (goto _label_4))))
                (:`CastFailed`
                  (`KismetSystemLibrary.PrintString` "Error castep" :!label _label_5)))
              (else
                (`KismetSystemLibrary.PrintString` "No valido" :!label _label_6))))
          (:`CastFailed`
            (bind _asabp_enemy (cast `/Game/Animations/Crypto/ABP_Enemy` _returnvalue)
              (:`then`
                (goto _label_3))
              (:`CastFailed`
                (`KismetSystemLibrary.PrintString` "anim instance fail")))))
        (else
          (goto _label_6))))
    (:`CastFailed`
      (goto _label_5))))