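; GA_Crouch is a Gameplay Ability that makes the avatar CharacterBase crouch for as long as the input is held.
; On activation it commits the ability, calls Crouch once the character and its movement component are valid, then waits for input release to end itself.
; UnCrouch runs in OnEndAbility, so the character is told to stand whenever the ability ends.
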(event `self.K2_ActivateAbility`
  (`self.K2_CommitAbility`)
  (bind _ascharacter_base (cast `CharacterBase` (`.AvatarActor` (break `GameplayAbilityActorInfo` (`self.GetActorInfo`)))))
  (if (and (`KismetSystemLibrary.IsValid` _ascharacter_base) (`KismetSystemLibrary.IsValid` (`Pawn.GetMovementComponent` _ascharacter_base)))
    (`Character.Crouch` _ascharacter_base)
    (`AbilityTask_WaitInputRelease.WaitInputRelease` false
      (:`OnRelease`
        (`self.K2_EndAbility`)))))

(event `self.K2_OnEndAbility`
  (params (bWasCancelled :type Boolean))
  (bind _ascharacter_base (cast `CharacterBase` (`.AvatarActor` (break `GameplayAbilityActorInfo` (`self.GetActorInfo`)))))
  (if (and (`KismetSystemLibrary.IsValid` _ascharacter_base) (`KismetSystemLibrary.IsValid` (`Pawn.GetMovementComponent` _ascharacter_base)))
    (`Character.UnCrouch` _ascharacter_base)))