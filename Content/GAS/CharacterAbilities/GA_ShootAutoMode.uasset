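; GA_ShootAutoMode is a Gameplay Ability that fires one hitscan shot from the owning avatar.
; After committing, it starts a sped-up shoot montage, then immediately line traces from the combat interface's socket along its target direction, with debug drawing on.
; A hit CharacterBase gets GE_Damage applied through its own ability system component.
; The ability ends after a completed trace and cancels if the montage is interrupted or cancelled.
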(event `self.K2_ActivateAbility`
  (bind (_returnvalue_owneractor _returnvalue_avataractor) (break `GameplayAbilityActorInfo` (`self.GetActorInfo`)))
  (`self.K2_CommitAbility`)
  (`AbilityTask_PlayMontageAndWait.CreatePlayMontageAndWaitProxy` "None" "/Game/Animations/Character/AM_Shoot.AM_Shoot" 3.0 "None" false
    (:`then`
      (bind _ascombat_interface (cast `CombatInterface` _returnvalue_avataractor))
      (bind _returnvalue (`CombatInterface.GetSocketLocation` _ascombat_interface))
      (bind _returnvalue_2 (`CombatInterface.GetTargetDirection` _ascombat_interface))
      (bind _outhit (`KismetSystemLibrary.LineTraceSingleForObjects` _returnvalue (+ _returnvalue (* _returnvalue_2 100000.0)) (`|MakeArray` "ObjectTypeQuery3" "ObjectTypeQuery1" "ObjectTypeQuery2" :!type "EObjectTypeQuery Enum") false (`|MakeArray` _returnvalue_avataractor) "ForDuration"))
      (bind _ascharacter_base (cast `CharacterBase` (`.HitActor` (`GameplayStatics.BreakHitResult` _outhit)))
        (:`then`
          (`AbilitySystemComponent.BP_ApplyGameplayEffectToSelf` :`self` (`AbilitySystemBlueprintLibrary.GetAbilitySystemComponent` _ascharacter_base) :`GameplayEffectClass` "/Game/GAS/GameplayEffects/GE_Damage.GE_Damage_C"))
        (:`CastFailed`
          _))
      (`self.K2_EndAbility`))
    (:`OnInterrupted`
      (`self.K2_CancelAbility` :!label _label))
    (:`OnCancelled`
      (goto _label))))