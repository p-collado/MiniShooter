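; GA_FireShoot is a gameplay ability that fires a hitscan shot from the avatar character.
; On activation it commits, plays AM_Shoot at increased rate and immediately line-traces for Pawns along the CombatUtils shoot position and direction, with debug drawing.
; A hit CharacterBase applies GE_Damage to itself through its own ability system component.
; The ability ends on montage completion or blend-out, and cancels on interruption.
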(event `self.K2_ActivateAbility`
  (bind (_returnvalue_owneractor _returnvalue_avataractor) (break `GameplayAbilityActorInfo` (`self.GetActorInfo`)))
  (`self.K2_CommitAbility`)
  (`AbilityTask_PlayMontageAndWait.CreatePlayMontageAndWaitProxy` "None" "/Game/Animations/Character/AM_Shoot.AM_Shoot" 3.0 "None" false
    (:`then`
      (bind _ascharacter_base (cast `CharacterBase` _returnvalue_avataractor))
      (bind (_combatutils_shootposition _combatutils_shootdirection) (break `CombatUtils` (`CharacterBase.CombatUtils` _ascharacter_base)))
      (bind _outhit (`KismetSystemLibrary.LineTraceSingleForObjects` _combatutils_shootposition (+ (* _combatutils_shootdirection 100000.0) _combatutils_shootposition) (`|MakeArray` "ObjectTypeQuery3" :!type "EObjectTypeQuery Enum") false (`|MakeArray` _returnvalue_avataractor) "ForDuration"))
      (bind _ascharacter_base_2 (cast `CharacterBase` (`.HitActor` (`GameplayStatics.BreakHitResult` _outhit))))
      (`AbilitySystemComponent.BP_ApplyGameplayEffectToSelf` :`self` (`AbilitySystemBlueprintLibrary.GetAbilitySystemComponent` _ascharacter_base_2) :`GameplayEffectClass` "/Game/GAS/GameplayEffects/GE_Damage.GE_Damage_C"))
    (:`OnCompleted`
      (`self.K2_EndAbility` :!label _label))
    (:`OnBlendOut`
      (goto _label))
    (:`OnInterrupted`
      (`KismetSystemLibrary.PrintString` "Cancelled" :!label _label_2)
      (`self.K2_CancelAbility`))
    (:`OnCancelled`
      (goto _label_2))))